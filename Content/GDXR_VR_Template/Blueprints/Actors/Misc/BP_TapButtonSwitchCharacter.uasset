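; Tap button actor that switches the VR player between the Quinn and Manny characters when its mesh is overlapped.
; An overlap triggers a game instance screen fade-out and saves the player's transform.
; When the fade completes, it destroys body-storage holster actors and the current player, spawns the selected character there, possesses the game instance's CurrentPlayer and flips the selection.
; A DoOnce blocks retriggering until fade-in completes.
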(event `self.StaticMesh.OnComponentBeginOverlap`
  (params (OverlappedComponent :type "PrimitiveComponent Object Reference") (OtherActor :type "Actor Object Reference") (OtherComp :type "PrimitiveComponent Object Reference") (OtherBodyIndex :type Integer) (bFromSweep :type Boolean) (SweepResult :type "HitResult Structure (by ref)"))
  (bind _returnvalue (`GameplayStatics.GetGameInstance`))
  (`/Engine/EditorBlueprintResources/StandardMacros.DoOnce` false :!label _label
    (:`Completed`
      ;[0.008681 0.008681 0.008681] Castr to game instance to get fade details
      (message `/Game/GDXR_VR_Template/Blueprints/Interfaces/BPI_ScreenFade.FadeOut` _returnvalue)
      (bind _asvr_game_instance (cast `/Game/GDXR_VR_Template/Blueprints/VR_GameInstance` _returnvalue))
      (set `self.As VR Game Instance` _asvr_game_instance)
      ;[0.008681 0.008681 0.008681] Once fade out completes change character
      (add `/Game/GDXR_VR_Template/Blueprints/VR_GameInstance.FadeOutComplete` (`self.As VR Game Instance`) (delegate `FadeOutComplete_Event`))
      (set `self.Get Player Transform` (`self.GetTransform` (`/Game/GDXR_VR_Template/Blueprints/VR_GameInstance.CurrentPlayer` (`self.As VR Game Instance`))))
      ;[0.008681 0.008681 0.008681] Once fade in completes let user change character again
      (add `/Game/GDXR_VR_Template/Blueprints/VR_GameInstance.FadeInComplete` (`self.As VR Game Instance`) (delegate `FadeInComplete_Event`)))))

(event `FadeInComplete_Event`
  ;[0.008681 0.008681 0.008681] Once fade in completes let user change character again
  (`self.Reset Do once`))

(event `Reset Do once`
  (goto _label :!via `Reset`))

(event `FadeOutComplete_Event`
  (bind _bodystorageactors (break `/Game/GDXR_VR_Template/Blueprints/Data/S_Inventory` (`/Game/GDXR_VR_Template/Blueprints/VR_GameInstance.InventoryStruct` (`self.As VR Game Instance`))))
  ;[0.008681 0.008681 0.008681] Destory Actors which spawned with the Holster actor
  (for _array_element _bodystorageactors
    (`self.K2_DestroyActor` _array_element))
  (`KismetArrayLibrary.Array_Clear` _bodystorageactors)
  ;[0.008681 0.008681 0.008681] Stops other actors using screen fade from making new players
  (remove `/Game/GDXR_VR_Template/Blueprints/VR_GameInstance.FadeOutComplete` (`self.As VR Game Instance`) (delegate `FadeOutComplete_Event`))
  ;[0.008681 0.008681 0.008681] Once fade out completes, Spawn the new character actor and posses it. Destroy the old one and change the character number.
  (`self.K2_DestroyActor` (`/Game/GDXR_VR_Template/Blueprints/VR_GameInstance.CurrentPlayer` (`self.As VR Game Instance`)))
  (`|SpawnActorFromClass` (select `int` (`self.CharacterToUse`) :`0` "/Game/GDXR_VR_Template/Blueprints/BP_VR_Character_Quinn.BP_VR_Character_Quinn_C" :`1` "/Game/GDXR_VR_Template/Blueprints/BP_VR_Character_Manny.BP_VR_Character_Manny_C" :!type "Actor Class Reference") (`self.Get Player Transform`) "AlwaysSpawn" "OverrideRootScale" null null)
  (`Controller.Possess` (`GameplayStatics.GetPlayerController` 0) (`/Game/GDXR_VR_Template/Blueprints/VR_GameInstance.CurrentPlayer` (`self.As VR Game Instance`)))
  (if (>= (`self.CharacterToUse`) 1)
    (set `self.CharacterToUse` 0)
    (else
      (set `self.CharacterToUse` 1))))

(fn `UserConstructionScript`)