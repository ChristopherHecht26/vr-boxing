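; BP_GazeInteraction is an actor that toggles gaze interaction for the VR player character.
; On BeginPlay it casts the player character to BP_VR_Character_Manny and caches it.
; Its Activation event uses a FlipFlop to alternately enable and disable gaze interaction in the character's CGazeInteraction component settings, showing or hiding the gaze interaction message to match.
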(event `self.ReceiveBeginPlay`
  (bind _asbp_vr_character_manny (cast `/Game/GDXR_VR_Template/Blueprints/BP_VR_Character_Manny` (`GameplayStatics.GetPlayerCharacter` 0)))
  (set `self.As BP VR Character` _asbp_vr_character_manny))

(event `/Game/GDXR_VR_Template/Blueprints/Interfaces/BPI_PlayerInteractions.Activation`
  (params (State :type Boolean))
  (bind _c_gazeinteraction (`/Game/GDXR_VR_Template/Blueprints/BP_VR_Character_Manny.C_GazeInteraction` (`self.As BP VR Character`)))
  (bind _gazeusersettings (`/Game/GDXR_VR_Template/Blueprints/Components/GazeInteraction/C_GazeInteraction.GazeUserSettings` _c_gazeinteraction))
  (`/Engine/EditorBlueprintResources/StandardMacros.FlipFlop`
    (:`A`
      (setmembers `/Game/GDXR_VR_Template/Blueprints/Data/S_GazeInteractionSettings` :`StructRef` _gazeusersettings :`Use Gaze Interaction` true :`Use Gaze interaction With UMG` true :`Permenantly Display Gaze Interaction` true :`Look Away To Restart Gaze Timer` false :`Gaze Line Trace Distance` 1000.0 :`Gaze icon Distance From Camera` 150.0 :`Gaze interaction Z Offset` 0.0 :`Gaze Interaction Timer Length` 2.0)
      (message `/Game/GDXR_VR_Template/Blueprints/Interfaces/BPI_GazeInteraction.DisplayGazeInteraction` _c_gazeinteraction))
    (:`B`
      (setmembers `/Game/GDXR_VR_Template/Blueprints/Data/S_GazeInteractionSettings` :`StructRef` _gazeusersettings :`Use Gaze Interaction` false :`Use Gaze interaction With UMG` true :`Permenantly Display Gaze Interaction` true :`Look Away To Restart Gaze Timer` false :`Gaze Line Trace Distance` 1000.0 :`Gaze icon Distance From Camera` 150.0 :`Gaze interaction Z Offset` 0.0 :`Gaze Interaction Timer Length` 2.0)
      (message `/Game/GDXR_VR_Template/Blueprints/Interfaces/BPI_GazeInteraction.HideGazeInteraction` _c_gazeinteraction))))

(fn `UserConstructionScript`)