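; BP_BodyHolster is a VR body holster actor that follows the player's body without inheriting head pitch or roll.
; When auto-attach is enabled, BeginPlay attaches it to player character 0 and starts a looping timer.
; Each tick of the timer eases the root's yaw toward the camera's and places it at the camera's horizontal position and the capsule's height, with sweep.
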(event `self.ReceiveBeginPlay`
  (bind _returnvalue (`GameplayStatics.GetPlayerCharacter` 0))
  (if (`self.AutoAttachToPlayer?`)
    (`/Engine/EditorBlueprintResources/StandardMacros.IsValid` _returnvalue
      (:`Is Valid`
        (`self.K2_AttachToActor` _returnvalue "None" "SnapToTarget" "SnapToTarget" "SnapToTarget")
        (bind _returnvalue_2 (`KismetSystemLibrary.K2_SetTimerDelegate` (delegate `Update Holster Rotation`) 0.02 true))))))

(event `Update Holster Rotation`
  (bind _returnvalue (`GameplayStatics.GetPlayerCharacter` 0))
  (bind _defaultsceneroot (`self.DefaultSceneRoot`))
  (bind _returnvalue_2 (`self.GetComponentByClass` _returnvalue "/Script/Engine.CameraComponent"))
  (bind (_returnvalue_x _returnvalue_y) (`KismetMathLibrary.BreakVector` (`SceneComponent.K2_GetComponentLocation` _returnvalue_2)))
  (bind (_returnvalue_x_2 _returnvalue_y_2 _returnvalue_z) (`KismetMathLibrary.BreakVector` (`SceneComponent.K2_GetComponentLocation` (`self.GetComponentByClass` _returnvalue "/Script/Engine.CapsuleComponent"))))
  (bind (_returnvalue_roll _returnvalue_pitch _returnvalue_yaw) (`KismetMathLibrary.BreakRotator` (`KismetMathLibrary.RInterpTo` (`SceneComponent.K2_GetComponentRotation` _defaultsceneroot) (`SceneComponent.K2_GetComponentRotation` _returnvalue_2) (`KismetSystemLibrary.K2_GetTimerElapsedTimeHandle` (stale `self.ReceiveBeginPlay` _returnvalue_2)) 2.0)))
  (`SceneComponent.K2_SetWorldRotation` _defaultsceneroot (`KismetMathLibrary.MakeRotator` 0.0 0.0 _returnvalue_yaw) false false)
  (`SceneComponent.K2_SetWorldLocation` _defaultsceneroot (`KismetMathLibrary.MakeVector` _returnvalue_x _returnvalue_y _returnvalue_z) true false))

(fn `UserConstructionScript`)